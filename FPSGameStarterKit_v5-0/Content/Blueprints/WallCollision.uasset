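; WallCollision is an indexed wall actor that belongs to a Room and shows its index on a TextRender.
; Update stores a new index and refreshes the displayed number, and BeginPlay calls it with the current value.
; RemoveIndex has the Room remove the wall at that index, then destroys this actor.
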(event `self.ReceiveBeginPlay`
  (`self.Update` (`self.Index`)))

(event `Update`
  (params (`New Index` :type Integer))
  (bind _output_get (set `self.Index` `New Index`))
  (`TextRenderComponent.K2_SetText` (`self.TextRender`) (`KismetTextLibrary.Conv_IntToText` _output_get)))

(event `RemoveIndex`
  (`/Game/Blueprints/BP_Room.Remove Wall` (`self.Room`) (`self.Index`))
  (`self.K2_DestroyActor`))

(fn `UserConstructionScript`)