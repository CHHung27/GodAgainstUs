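; Procedural dungeon door that swings open on Activate and, if Roomify is set, generates the room or hall behind it.
; A seeded random stream drives sizes, shift, door counts and child seeds.
; Line traces probe free space: hitting a door or wall collision spawns a connecting hall BP_Room, while no hit spawns a room fitted between side limits.
; The right-side trace result is unwired, so RightLimit drops to zero.
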(event `self.ReceiveBeginPlay`
  (set `self.DoorStream` (`KismetMathLibrary.MakeRandomStream` (`self.Seed`))))

(event `/Game/Blueprints/BPI_Activate.Activate`
  (if (`self.Closed`)
    (set `self.Closed` false)
    (`|ExecutionSequence`
      (:`then_0`
        (if (`self.Roomify`)
          (set `self.Roomify` false)
          (bind _output_get (set `self.Room Size Limit` (`KismetMathLibrary.RandomIntegerInRangeFromStream` 2 7 (`self.DoorStream`))))
          (bind _output_get_2 (set `self.Left Limit` _output_get))
          (set `self.Right Limit` _output_get_2)
          (`self.AddAddition`)))
      (:`then_1`
        (bind (_direction _dooryaw) (`Timeline|OpenDoorTimeline`)
          (:`Update`
            (`SceneComponent.K2_SetRelativeRotation` (`self.Hinge`) (`KismetMathLibrary.MakeRotator` 0.0 0.0 _dooryaw) false false)))))))

(event `New Room`
  (params (`Room Tiles X` :type Integer) (`Room TIles Y` :type Integer) (Shift :type Integer) (`Max Doors` :type Integer) (Hall :type Boolean))
  (`|SpawnActorFromClass` "/Game/Blueprints/BP_Room.BP_Room_C" (`KismetMathLibrary.MakeTransform` (+ (`self.K2_GetActorLocation`) (* (`self.GetActorForwardVector`) 400.0)) (`KismetMathLibrary.ComposeRotators` (`self.K2_GetActorRotation`) (struct :`Yaw` 90.0))) "Undefined" "OverrideRootScale" null `Room Tiles X` `Room TIles Y` `Max Doors` Shift Hall (`KismetMathLibrary.RandomIntegerFromStream` 100000 (`self.DoorStream`)) null))

(event `AddAddition`
  (bind _space (`self.Space`))
  (bind _returnvalue (`KismetMathLibrary.TransformLocation` (`self.GetTransform`) (200.0 10.0 200.0)))
  (bind _returnvalue_2 (* (`self.GetActorForwardVector`) (+ (* (- (`self.Room Size Limit`) 1) (`self.TileSize`)) 10.0)))
  (bind (_outhit _returnvalue_3) (`KismetSystemLibrary.LineTraceSingle` :`Start` _returnvalue :`End` (+ _returnvalue (* (`self.GetActorRightVector`) (* (`self.Room Size Limit`) (`self.TileSize`)))) :`TraceChannel` "TraceTypeQuery1" :`DrawDebugType` "Persistent"))
  (if _returnvalue_3
    (bind (_bblockinghit _binitialoverlap _time _distance _location _impactpoint _normal _impactnormal _physmat _hitactor) (`GameplayStatics.BreakHitResult` _outhit))
    (switch `string` (`KismetSystemLibrary.GetClassDisplayName` (`GameplayStatics.GetObjectClass` _hitactor))
      (:`BP_Door_C`
        (bind _asbp_door (cast `/Game/Blueprints/BP_Door` _hitactor))
        (set `/Game/Blueprints/BP_Door.Roomify` false _asbp_door))
      (:`WallCollision_C`
        (bind _aswall_collision (cast `/Game/Blueprints/WallCollision` _hitactor))
        (`/Game/Blueprints/WallCollision.RemoveIndex` _aswall_collision)))
    (`self.New Room` (`KismetMathLibrary.Round` (/ _distance (`self.TileSize`))) 1 0 (`KismetMathLibrary.RandomIntegerInRangeFromStream` 0 2 (`self.DoorStream`)) true)
    (else
      (for _index (range (`self.Room Size Limit`))
        ;[1 1 1] Left limit check
        (`|ExecutionSequence`
          (:`then_0`
            (bind _returnvalue_4 (`KismetMathLibrary.TransformLocation` (`self.GetTransform`) (+ (390.0 200.0 300.0) (`KismetMathLibrary.MakeVector` 0.0 (* _index 400.0)))))
            (bind (_outhit_2 _returnvalue_5) (`KismetSystemLibrary.LineTraceSingle` :`Start` _returnvalue_4 :`End` (+ _returnvalue_4 _returnvalue_2) :`TraceChannel` "TraceTypeQuery1" :`DrawDebugType` "Persistent"))
            (if _returnvalue_5
              (set `self.Left Limit` (`KismetMathLibrary.Min` (`KismetMathLibrary.Round` (/ (`.Distance` (`GameplayStatics.BreakHitResult` _outhit_2)) (`self.TileSize`))) (`self.Left Limit`)))))
          (:`then_1`
            (bind _returnvalue_6 (`KismetMathLibrary.TransformLocation` (`self.GetTransform`) (+ (10.0 200.0 300.0) (`KismetMathLibrary.MakeVector` 0.0 (* _index 400.0)))))
            ;[1 1 1] Right limit check
            (bind _outhit_3 (`KismetSystemLibrary.LineTraceSingle` :`Start` _returnvalue_6 :`End` (+ _returnvalue_6 (* _returnvalue_2 -1.0)) :`TraceChannel` "TraceTypeQuery1" :`DrawDebugType` "Persistent"))
            (if true
              (set `self.Right Limit` (`KismetMathLibrary.Min` (`KismetMathLibrary.Round` (/ 0.0 (`self.TileSize`))) (`self.Right Limit`)))))))
      ;[1 1 1] set available space
      (set `self.Space` (`KismetMathLibrary.RandomIntegerInRangeFromStream` 0 (`KismetMathLibrary.Min` (+ (`self.Right Limit`) (`self.Left Limit`)) (`self.Room Size Limit`)) (`self.DoorStream`)))
      ;[1 1 1] get room shift to fit available space
      (set `self.Shift` (`KismetMathLibrary.RandomIntegerInRangeFromStream` (`KismetMathLibrary.Clamp` (- (`self.Space`) (`self.Right Limit`)) 0 _space) (`KismetMathLibrary.Min` _space (`self.Left Limit`)) (`self.DoorStream`)))
      ;[1 1 1] Spawn New Room
      (`self.New Room` (`KismetMathLibrary.RandomIntegerInRangeFromStream` 3 (`self.Room Size Limit`) (`self.DoorStream`)) (+ (`self.Space`) 1) (`self.Shift`) (`KismetMathLibrary.RandomIntegerInRangeFromStream` 1 3 (`self.DoorStream`))))))

(event `self.InteractPopup.OnComponentBeginOverlap`
  (params (OverlappedComponent :type "PrimitiveComponent Object Reference") (OtherActor :type "Actor Object Reference") (OtherComp :type "PrimitiveComponent Object Reference") (OtherBodyIndex :type Integer) (bFromSweep :type Boolean) (SweepResult :type "HitResult Structure (by ref)"))
  (cast `/Game/FirstPerson/Blueprints/BP_FirstPersonCharacter` OtherActor)
  (if (`self.Closed`)
    (`KismetSystemLibrary.PrintString` "Press E to open")))

(fn `UserConstructionScript`)