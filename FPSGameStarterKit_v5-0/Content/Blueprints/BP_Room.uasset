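; BP_Room procedurally builds a seeded, tile-based room or hall at BeginPlay from instanced floor and wall meshes.
; BasicRoom walks the grid and perimeter, leaving an entry gap for non-origin rooms and letting WallOrDoor randomly place seeded BP_Doors at regular intervals.
; Line traces skip occupied edges and clear Roomify on doors they hit.
; Each wall gets a WallCollision actor, and RemoveWall swap-removes these to match instance indices.
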(event `self.ReceiveBeginPlay`
  ;[1 1 1] Random Seed
  (set `self.RoomStream` (`KismetMathLibrary.MakeRandomStream` (`self.Seed`)))
  (`self.Basic Room`))

(event `Remove Wall`
  (params (Index :type Integer))
  (bind _wall_collisions (`self.Wall Collisions`))
  (bind _returnvalue (`KismetArrayLibrary.Array_LastIndex` _wall_collisions))
  (bind _output (`|GetArrayItem` _wall_collisions _returnvalue))
  (`InstancedStaticMeshComponent.RemoveInstance` (`self.Wall2`) Index)
  ;[1 1 1] Update collisions array to match wall instance array
  (`KismetArrayLibrary.Array_Set` _wall_collisions Index _output)
  (`/Game/Blueprints/WallCollision.Update` _output Index)
  (`KismetArrayLibrary.Array_Remove` (`self.Wall Collisions`) _returnvalue))

(fn `Basic Room`
  ;[1 1 1] Rows
  (for _index (range (`self.RoomTilesY`))
    ;[1 1 1] Columns
    (for _index_2 (range (`self.RoomTilesX`))
      ;[1 1 1] Spawn Floors
      (`InstancedStaticMeshComponent.AddInstance` (`self.Floor`) (`KismetMathLibrary.MakeTransform` (`KismetMathLibrary.MakeVector` (* _index_2 (`self.TileSizeX`)) (* (`self.TileSizeY`) (- _index (`self.Entry Shift`))))) false)))
  (if (not (`self.Hall`))
    (for _index_3 (range (`self.RoomTilesY`))
      ;[1 1 1] Bottom Wall
      ;;[1 1 1] Entry way check
      (if (or (`self.Origin`) (!= _index_3 (`self.Entry Shift`)))
        (bind _returnvalue (== (mod _index_3 (`self.Door Every`)) (`self.Door Remainder`)))
        (`self.WallOrDoor` _returnvalue (- (`KismetMathLibrary.MakeVector` 0.0 (* (`self.TileSizeY`) _index_3)) (`KismetMathLibrary.MakeVector` 0.0 (* (`self.Entry Shift`) (`self.TileSizeY`)))) (struct :`Yaw` 90.0)))
      ;[1 1 1] Top Wall
      (`self.WallOrDoor` _returnvalue (- (`KismetMathLibrary.MakeVector` (* (`self.RoomTilesX`) (`self.TileSizeX`)) (* (`self.TileSizeY`) (+ _index_3 1))) (`KismetMathLibrary.MakeVector` 0.0 (* (`self.Entry Shift`) (`self.TileSizeY`)))) (struct :`Yaw` -90.0))))
  (for _index_4 (range (`self.RoomTilesX`))
    (bind _returnvalue_2 (== (mod _index_4 (`self.Door Every`)) (`self.Door Remainder`)))
    ;[1 1 1] Right Wall
    (`self.WallOrDoor` _returnvalue_2 (- (`KismetMathLibrary.MakeVector` (* (`self.TileSizeX`) _index_4) (* (`self.TileSizeY`) (`self.RoomTilesY`))) (`KismetMathLibrary.MakeVector` 0.0 (* (`self.Entry Shift`) (`self.TileSizeY`)))))
    ;[1 1 1] Left Wall
    (`self.WallOrDoor` _returnvalue_2 (- (`KismetMathLibrary.MakeVector` (* (`self.TileSizeX`) (+ _index_4 1))) (`KismetMathLibrary.MakeVector` 0.0 (* (`self.Entry Shift`) (`self.TileSizeY`)))) (struct :`Yaw` 180.0))))

(fn `UserConstructionScript`)

(fn `WallOrDoor`
  (params (CanDoor :type Boolean) (`Instance Transform Location` :type "Vector Structure") (`Instance Transform Rotation` :type "Rotator Structure"))
  (bind _returnvalue (`self.GetTransform`))
  (bind _doorcount (`self.DoorCount`))
  (bind _returnvalue_2 (`KismetMathLibrary.TransformLocation` _returnvalue `Instance Transform Location`))
  (bind _returnvalue_3 (`KismetMathLibrary.TransformRotation` _returnvalue `Instance Transform Rotation`))
  (`self.CheckForWall` `Instance Transform Location` `Instance Transform Rotation`
    (:`false`
      ;[1 1 1] Is this a door
      (if (and CanDoor (`KismetMathLibrary.RandomBoolWithWeightFromStream` (`KismetMathLibrary.Conv_IntToDouble` (/ _doorcount (- _doorcount (`KismetArrayLibrary.Array_Length` (`self.Doors`))))) (`self.RoomStream`)))
        ;[1 1 1] Transform location and rotation to world space, spawn door, and add door to array
        (bind _returnvalue_4 (`|SpawnActorFromClass` "/Game/Blueprints/BP_Door.BP_Door_C" (`KismetMathLibrary.MakeTransform` _returnvalue_2 _returnvalue_3) "Undefined" "OverrideRootScale" null (`KismetMathLibrary.RandomIntegerFromStream` 10000 (`self.RoomStream`)) null))
        (`KismetArrayLibrary.Array_Add` (`self.Doors`) _returnvalue_4)
        (else
          (bind _returnvalue_5 (`InstancedStaticMeshComponent.AddInstance` (`self.Wall2`) (`KismetMathLibrary.MakeTransform` `Instance Transform Location` `Instance Transform Rotation`) false))
          (bind _returnvalue_6 (`|SpawnActorFromClass` "/Game/Blueprints/WallCollision.WallCollision_C" (`KismetMathLibrary.MakeTransform` _returnvalue_2 _returnvalue_3) "Undefined" "OverrideRootScale" null _returnvalue_5 self null))
          (`KismetArrayLibrary.Array_AddUnique` (`self.Wall Collisions`) _returnvalue_6))))))