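; AI Director actor that spawns zombies around the player and tracks wave completion.
; On BeginPlay it spawns AI_Zombie pawns running BT_Zombie at random reachable points within its influence radius, up to a maximum.
; Each tick it hovers above the player and compares the character's kill count to the wave size, incrementing the wave when met.
; Later waves spawn nothing, the reset misses the character's counter, and difficulty scaling is unfinished.
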(event `self.ReceiveAnyDamage`
  (params (Damage :type "Float (single-precision)") (DamageType :type "DamageType Object Reference") (InstigatedBy :type "Controller Object Reference") (DamageCauser :type "Actor Object Reference")))

(event `self.ReceiveBeginPlay`
  ;[1 1 1] TODO: Spawn Zombie event (within director sphere of influence and ////optionally out of sight of player)
  (while (< (`self.NumberOfZombies`) (`self.MaxNumberOfZombie`))
    (`self.Summon Zombie`))
  (`KismetSystemLibrary.PrintString` "Wave Spawned"))

(event `self.ReceiveTick`
  (params (DeltaSeconds :type "Float (single-precision)"))
  (bind (_returnvalue_x _returnvalue_y _returnvalue_z) (`KismetMathLibrary.BreakVector` (`self.K2_GetActorLocation` (`GameplayStatics.GetPlayerCharacter` 0))))
  ;[1 1 1] On event tick, update director location to follow player
  (`self.K2_SetActorLocation` (`KismetMathLibrary.MakeVector` _returnvalue_x _returnvalue_y (+ _returnvalue_z 400.0)))
  ;[1 1 1] Checking if wave is complete based on player kills
  (bind _asbp_character_base (cast `/Game/GodAgainstUs/Blueprints/BP_CharacterBase` (`GameplayStatics.GetPlayerCharacter` 0)))
  (if (< (`/Game/GodAgainstUs/Blueprints/BP_CharacterBase.zombieKilled` _asbp_character_base) (`self.ZombiesInWave`))
    (`KismetSystemLibrary.PrintString` "Wave Not Cleared" true true (struct :`G` 0.66 :`B` 1.0 :`A` 1.0) 0.0)
    (else
      (`KismetSystemLibrary.PrintString` "Wave Cleared!" true true (struct :`G` 0.66 :`B` 1.0 :`A` 1.0) 0.0)
      ;[1 1 1] add one to current wave, reset zombie kills to zero, TODO: delay until the next wave starts
      (`/Engine/EditorBlueprintResources/StandardMacros.IncrementInt` (`self.WaveNumber`)
        (:`  `
          (set `self.ZombiesKilled` 0))))))

(fn `Summon Zombie`
  (`AIBlueprintHelperLibrary.SpawnAIFromClass` "/Game/GodAgainstUs/Blueprints/Zombie/AI_Zombie.AI_Zombie_C" "/Game/GodAgainstUs/Blueprints/Zombie/BT_Zombie.BT_Zombie" (`NavigationSystemV1.K2_GetRandomReachablePointInRadius` (`self.K2_GetActorLocation` self) (`KismetMathLibrary.Conv_IntToDouble` (`self.SphereOfInfluenceRadius`)) null null) (struct) false null)
  (`/Engine/EditorBlueprintResources/StandardMacros.IncrementInt` (`self.NumberOfZombies`)))

(fn `UserConstructionScript`)