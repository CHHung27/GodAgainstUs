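; Behavior tree task that moves a zombie to the actor stored in its TargetActorToFollow blackboard key.
; It casts the owner to AI_Con_Zombie, caches that controller, and runs AIMoveTo on the controlled pawn with a small acceptance radius.
; Success finishes the task, while failure clears the target key without calling FinishExecute.
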(event `self.ReceiveExecute`
  (params (OwnerActor :type "Actor Object Reference"))
  (`/Engine/EditorBlueprintResources/StandardMacros.IsValid` (`self.Zombie_Controller`)
    (:`Is Valid`
      _)
    (:`Is Not Valid`
      (bind _asai_con_zombie (cast `/Game/GodAgainstUs/Blueprints/Zombie/AI_Con_Zombie` OwnerActor))
      (set `self.Zombie_Controller` _asai_con_zombie)))
  (`|AIMoveTo` (`Controller.K2_GetPawn` (`self.Zombie_Controller`)) (0.0 0.0 0.0) (`BTFunctionLibrary.GetBlackboardValueAsActor` (`self.TargetActorToFollow`)) 10.0
    (:`OnSuccess`
      (`self.FinishExecute` true))
    (:`OnFail`
      (`BTFunctionLibrary.SetBlackboardValueAsObject` (`self.TargetActorToFollow`)))))