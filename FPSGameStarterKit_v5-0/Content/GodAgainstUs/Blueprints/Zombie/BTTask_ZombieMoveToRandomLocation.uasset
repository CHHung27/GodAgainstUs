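; Behaviour tree task that makes a zombie wander to a random navigable point around its current location.
; It caches the AI_Con_Zombie controller, writes a random point to the RandomLocation blackboard key and runs AIMoveTo on the pawn.
; The random-point lookup is evaluated separately for each, so the stored key can differ from the actual destination.
; The task always finishes as successful, after a short delay if the move fails.
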(event `self.ReceiveExecute`
  (params (OwnerActor :type "Actor Object Reference"))
  (bind _returnvalue (`Controller.K2_GetPawn` (`self.Zombie_Con_Ref`)))
  (bind _randomlocation (`NavigationSystemV1.K2_GetRandomLocationInNavigableRadius` (`Actor.K2_GetActorLocation` _returnvalue) 1000.0 null null))
  (`/Engine/EditorBlueprintResources/StandardMacros.IsValid` (`self.Zombie_Con_Ref`)
    (:`Is Valid`
      _)
    (:`Is Not Valid`
      (bind _asai_con_zombie (cast `/Game/GodAgainstUs/Blueprints/Zombie/AI_Con_Zombie` OwnerActor))
      (set `self.Zombie_Con_Ref` _asai_con_zombie)))
  (`BTFunctionLibrary.SetBlackboardValueAsVector` (`self.RandomLocation`) _randomlocation)
  (`|AIMoveTo` _returnvalue _randomlocation null 50.0
    (:`OnSuccess`
      (`self.FinishExecute` true))
    (:`OnFail`
      (`KismetSystemLibrary.Delay` 2.0)
      (`self.FinishExecute` true))))