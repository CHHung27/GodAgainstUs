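; Behavior tree decorator for zombie AI that gates a branch on how far the zombie is from the actor it follows.
; It casts the owner to AI_Con_Zombie and reads the follow target from the TargetActorToFollow blackboard key.
; The condition passes when the straight-line distance between the controlled pawn and that target is at least the Distance threshold, despite the "Reached" in its name.
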(fn `PerformConditionCheck`
  (params (OwnerActor :type "Actor Object Reference"))
  (returns (ReturnValue :type Boolean))
  (bind _asai_con_zombie (cast `/Game/GodAgainstUs/Blueprints/Zombie/AI_Con_Zombie` OwnerActor))
  (set `self.Zombie_Controller` _asai_con_zombie)
  (return (>= (`KismetMathLibrary.VSize` (- (`Actor.K2_GetActorLocation` (`BTFunctionLibrary.GetBlackboardValueAsActor` (`self.TargetActorToFollow`))) (`Actor.K2_GetActorLocation` (`Controller.K2_GetPawn` (`self.Zombie_Controller`))))) (`self.Distance`))))