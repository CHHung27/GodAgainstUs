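; AI controller for the zombie enemy, driving it through Blackboard_Zombie and the BT_Zombie behavior tree.
; On BeginPlay it waits briefly to avoid a Spawn AI From Class error, stores the pawn's location as HomeLocation, starts the tree and caches the zombie character.
; AttackPlayer calls AttachPlayerChar on that zombie when the blackboard's TargetActorToFollow is valid.
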(event `self.ReceiveBeginPlay`
  (`self.UseBlackboard` "/Game/GodAgainstUs/Blueprints/Zombie/Blackboard_Zombie.Blackboard_Zombie")
  (`KismetSystemLibrary.Delay` 0.2) ; This delay is needed to prevent an error when using the Spawn AI From Class node
  (`BlackboardComponent.SetValueAsVector` (`AIBlueprintHelperLibrary.GetBlackboard` self) (`self.HomeLocation`) (`self.K2_GetActorLocation` (`self.K2_GetPawn`)))
  (`self.RunBehaviorTree` "/Game/GodAgainstUs/Blueprints/Zombie/BT_Zombie.BT_Zombie")
  (bind _asbp_ai_char_zombie (cast `/Game/GodAgainstUs/Blueprints/Zombie/BP_AI_CharZombie` (`self.K2_GetPawn`)))
  (set `self.ZombieCast` _asbp_ai_char_zombie))

(event `AttackPlayer`
  (`/Engine/EditorBlueprintResources/StandardMacros.IsValid` (`BlackboardComponent.GetValueAsObject` (`AIBlueprintHelperLibrary.GetBlackboard` self) (`self.TargetActorToFollow`))
    (:`Is Valid`
      (`/Game/GodAgainstUs/Blueprints/Zombie/BP_AI_CharZombie.AttachPlayerChar` (`self.ZombieCast`)))))

(fn `UserConstructionScript`)