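; Behavior Tree service that gives zombies aggro by detecting visible targets around the controlled pawn on each tick.
; It caches the zombie AI controller, then sphere-traces a large radius for the desired object types, ignoring all zombie characters.
; Each hit gets a Camera-channel line-of-sight trace that writes target actor and location to the Blackboard, or clears the target if blocked.
; The loop never breaks, so the last hit evaluated decides the target.
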(event `self.ReceiveTickAI`
  (params (OwnerController :type "AIController Object Reference") (ControlledPawn :type "Pawn Object Reference") (DeltaSeconds :type "Float (single-precision)"))
  (bind _targetactortofollow (`self.TargetActorToFollow`))
  (bind _returnvalue (`Actor.K2_GetActorLocation` (`Controller.K2_GetPawn` (`self.Zombie_Controller`))))
  (`/Engine/EditorBlueprintResources/StandardMacros.IsValid` (`self.Zombie_Controller`)
    (:`Is Valid`
      _)
    (:`Is Not Valid`
      (bind _asai_con_zombie (cast `/Game/GodAgainstUs/Blueprints/Zombie/AI_Con_Zombie` OwnerController))
      (set `self.Zombie_Controller` _asai_con_zombie)))
  (bind _outactors (`GameplayStatics.GetAllActorsOfClass` "/Game/GodAgainstUs/Blueprints/Zombie/BP_AI_CharZombie.BP_AI_CharZombie_C"))
  (set `self.AI_Location` _returnvalue)
  (bind _outhits (`KismetSystemLibrary.SphereTraceMultiForObjects` _returnvalue (+ _returnvalue (0.0 0.0 15.0)) 1500.0 (`self.DesiredObjectTypes`) false _outactors))
  (for _array_element _outhits
    (bind (_bblockinghit _binitialoverlap _time _distance _location _impactpoint _normal _impactnormal _physmat _hitactor) (`GameplayStatics.BreakHitResult` _array_element))
    (bind _outhit (`KismetSystemLibrary.LineTraceSingle` (`self.AI_Location`) (`Actor.K2_GetActorLocation` _hitactor) "TraceTypeQuery2" false _outactors))
    (bind (_bblockinghit_2 _binitialoverlap_2 _time_2 _distance_2 _location_2 _impactpoint_2 _normal_2 _impactnormal_2 _physmat_2 _hitactor_2) (`GameplayStatics.BreakHitResult` _outhit))
    (if (== _hitactor_2 _hitactor)
      (`BTFunctionLibrary.SetBlackboardValueAsObject` _targetactortofollow _hitactor_2)
      (`BTFunctionLibrary.SetBlackboardValueAsVector` (`self.PlayerLocationKey`) (`Actor.K2_GetActorLocation` _hitactor_2))
      (else
        (`BTFunctionLibrary.SetBlackboardValueAsObject` _targetactortofollow)))))