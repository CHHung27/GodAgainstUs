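; Health pickup that either heals the player or is stored for later use.
; Interaction caches the character in PlayerCast and shares the use-item check: below max health it heals and destroys itself, otherwise it calls StoreThisItem, with an optional sound.
; Overlap by a hurt BP_CharacterBase jumps straight to the heal branch, which targets PlayerCast rather than the overlapping character.
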(event `/Game/FPS_Game/Blueprints/Inventory/BPI_ItemInterface.BPI_UseItem`
  (bind _playercast (`self.PlayerCast`))
  (`/Engine/EditorBlueprintResources/StandardMacros.CompareFloat` (`/Game/GodAgainstUs/Blueprints/BP_CharacterBase.HealthCurrent` _playercast) (`/Game/GodAgainstUs/Blueprints/BP_CharacterBase.HealthMax` _playercast) :!label _label
    (:`>`
      (`self.StoreThisItem` :!label _label_2)
      (if (`self.PlayInteractionSound`)
        (`GameplayStatics.SpawnSoundAtLocation` (`self.HealthSound`) (`self.K2_GetActorLocation`) (struct) 1.0 1.0 0.0 null null)))
    (:`==`
      (goto _label_2))
    (:`<`
      (`/Game/GodAgainstUs/Blueprints/BP_CharacterBase.HealthHeal` (`self.PlayerCast`) (`self.HealthToAdd`) :!label _label_3)
      (if (`self.PlayInteractionSound`)
        (`GameplayStatics.SpawnSoundAtLocation` (`self.HealthSound`) (`self.K2_GetActorLocation`) (struct) 1.0 1.0 0.0 null null))
      (`self.K2_DestroyActor`))))

(event `/Game/FPS_Game/Blueprints/System/BPI_Interact.BPI_Interaction`
  (params (CharacterReference :type "/Game/GodAgainstUs/Blueprints/BP_CharacterBase Object Reference"))
  (set `self.PlayerCast` CharacterReference)
  (goto _label))

(event `self.ReceiveActorBeginOverlap`
  (params (OtherActor :type "Actor Object Reference"))
  (bind _asbp_character_base (cast `/Game/GodAgainstUs/Blueprints/BP_CharacterBase` OtherActor))
  (if (< (`/Game/GodAgainstUs/Blueprints/BP_CharacterBase.HealthCurrent` _asbp_character_base) (`/Game/GodAgainstUs/Blueprints/BP_CharacterBase.HealthMax` _asbp_character_base))
    (goto _label_3)))

(fn `UserConstructionScript`)