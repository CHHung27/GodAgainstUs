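; Course exercise point light actor with a per-instance configurable look and a randomized strength and color at play start.
; Construction Script applies shadows, intensity and color from the LightProperty struct, using an enum to pick a specific or random list color.
; BeginPlay's custom event calls FnGetRandomValue, which maps a random array key to a label, intensity and color, prints the label and overrides the light.
; Disconnected tutorial snippets demonstrate arrays, loops, flow control and earlier light setups.
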(event `self.ReceiveBeginPlay`
  ;[1 1 1] V9 - This block calls the custom event that we created
  (`self.evGetRandomValue`))

(event `evGetRandomValue`
  (bind _pointlight (`self.PointLight`))
  ;[1 1 1] V9 - This is a custom event created
  ;[1 1 1] V9 - Function Get Random Value
  (bind (_output_string _intensity _color) (`self.fnGetRandomValue` (`self.MyArray`)))
  (`KismetSystemLibrary.PrintString` _output_string true true (struct :`G` 0.66 :`B` 1.0 :`A` 1.0) 5.0)
  (`LightComponent.SetIntensity` _pointlight _intensity)
  (`LightComponent.SetLightColor` _pointlight _color true))

(fn `fnGetRandomValue`
  (params (`Input Array` :type "Array of String"))
  (returns (`Output String` :type String) (Intensity :type "Float (double-precision)") (Color :type "LinearColor Structure"))
  (locals (StringSelection :type String) (LightIntensity :type "Float (double-precision)") (LightColor :type "LinearColor Structure"))
  (`|ExecutionSequence`
    (:`then_0`
      (switch `string` (`KismetArrayLibrary.Array_Random` `Input Array`)
        (:`Default`
          (set `local.StringSelection` "No Item Found")
          (set `local.LightIntensity` 0.0)
          (set `local.LightColor` (struct :`G` 1.0 :`B` 0.227447 :`A` 1.0)))
        (:`Key 1`
          (set `local.StringSelection` "Weak")
          (set `local.LightIntensity` 500.0)
          (set `local.LightColor` (struct :`R` 1.0 :`B` 0.205412 :`A` 1.0)))
        (:`Key 2`
          (set `local.StringSelection` "Medium")
          (set `local.LightIntensity` 5000.0)
          (set `local.LightColor` (struct :`R` 1.0 :`G` 0.961734 :`A` 1.0)))
        (:`Key 3`
          (set `local.StringSelection` "Strong")
          (set `local.LightIntensity` 50000.0)
          (set `local.LightColor` (struct :`R` 0.224284 :`B` 1.0 :`A` 1.0)))))
    (:`then_1`
      (return (`local.StringSelection`) (`local.LightIntensity`) (`local.LightColor`)))))

(fn `UserConstructionScript`
  (bind (_castsshadows _lightintensity _coloroptions) (break `/Game/_Course/Struc_LightProperty` (`self.Light Property`)))
  (bind (_colormethod _specificcolor _colorlist) (break `/Game/_Course/Struc_LightColor` _coloroptions))
  ;[1 1 1] V8 - Using an enum (ColorMethods) and a structure (Color Options) we can now change the color of each instance of the point light
  (`LightComponentBase.SetCastShadows` (`self.PointLight`) _castsshadows)
  (`LightComponent.SetIntensity` (`self.PointLight`) _lightintensity)
  (switch `/Game/_Course/Enum_ColorOptions` _colormethod
    (:`NewEnumerator0`
      (`LightComponent.SetLightColor` (`self.PointLight`) _specificcolor true))
    (:`NewEnumerator1`
      (`LightComponent.SetLightColor` (`self.PointLight`) (`KismetArrayLibrary.Array_Random` _colorlist) true))))