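; BP_Platform is a moving platform from a course Timeline showcase that shuttles its Cube between a start and end location.
; After an initial delay, a Timeline with adjustable play rate drives a vector Lerp on the relative location.
; On finish, it checks direction, waits a stop time, then reverses or replays to loop.
; A disconnected manual Lerp version and unused VInterp nodes remain in the graph.
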(event `self.ReceiveBeginPlay`
  ;[1 1 1] Video 11 - Timeline showcase
  (set `self.StartLocation` (`SceneComponent.RelativeLocation` (`self.Cube`)))
  (`TimelineComponent.SetPlayRate` (`self.TM_Movement`) (`self.Playrate`))
  (`KismetSystemLibrary.Delay` (`self.InitialDelay`))
  (`self.GoForward`))

(event `GoForward`
  (bind _platformstoptime (`self.PlatformStopTime`))
  ;[1 1 1] Video 11 - Timeline showcase
  (bind (_direction _alpha) (`Timeline|TM_Movement` :!label _label)
    (:`Update`
      (`SceneComponent.K2_SetRelativeLocation` (`self.Cube`) (`KismetMathLibrary.VLerp` (`self.StartLocation`) (`self.EndLocation`) _alpha) false false))
    (:`Finished`
      (if (`|EnumEquality` _direction "Forward")
        (`KismetSystemLibrary.Delay` _platformstoptime)
        (`self.GoBackward`)
        (else
          (`KismetSystemLibrary.Delay` _platformstoptime)
          (`self.GoForward`))))))

(event `GoBackward`
  ;[1 1 1] Video 11 - Timeline showcase
  (goto _label :!via `Reverse`))

(event `self.ReceiveTick`
  (params (DeltaSeconds :type "Float (single-precision)")))

(fn `UserConstructionScript`)